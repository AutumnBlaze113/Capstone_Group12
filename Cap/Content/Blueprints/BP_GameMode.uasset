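; BP_GameMode is the game mode that sets a difficulty-based time limit and handles the two losing conditions.
; On BeginPlay it reads GameDifficulty from BP_GameInstance and sets CurrentTime, with less time on harder settings.
; Each Tick it opens the Timeup level when time runs out, otherwise the Death level if the ThirdPersonCharacter's Health equals zero.
; CurrentTime is only initialized and checked here, not counted down.
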(event `self.ReceiveBeginPlay`
  (bind _asbp_game_instance (cast `/Game/Blueprints/BP_GameInstance` (`GameplayStatics.GetGameInstance`)))
  (switch `/Game/Blueprints/BP_EDifficultyLevel` (`/Game/Blueprints/BP_GameInstance.GameDifficulty` _asbp_game_instance)
    (:`NewEnumerator0`
      (set `self.currentTime` 500.0))
    (:`NewEnumerator1`
      (set `self.currentTime` 300.0))
    (:`NewEnumerator2`
      (set `self.currentTime` 200.0))
    (:`NewEnumerator3`
      (set `self.currentTime` 90.0))))

(event `self.ReceiveTick`
  (params (DeltaSeconds :type "Float (single-precision)"))
  (if (<= (`self.currentTime`) 0.0)
    (`GameplayStatics.OpenLevel` "Timeup")
    (else
      (bind _asthird_person_character (cast `/Game/ThirdPersonCPP/Blueprints/ThirdPersonCharacter` (`GameplayStatics.GetPlayerCharacter` 0)))
      (if (== (`CapCharacter.health` _asthird_person_character) 0)
        (`GameplayStatics.OpenLevel` "Death")))))

(fn `UserConstructionScript`)