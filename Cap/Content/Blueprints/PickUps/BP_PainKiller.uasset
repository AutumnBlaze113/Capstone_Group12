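; BP_PainKiller is an interactable pickup that adds one to the player CapCharacter's Vaccine count, then destroys itself.
; Box overlap enables input on the actor, shows a PickupWidget2 prompt and opens a gate, while end overlap reverses all three.
; The Pickup input only passes through the open gate.
; Overlap events cast player character 0 without checking which actor overlapped.
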(event `InputAction|Pickup`
  (params (Key :type "Key Structure"))
  (:`Pressed`
    (`/Engine/EditorBlueprintResources/StandardMacros.Gate` true :!label _label
      (:`Exit`
        (`/Engine/EditorBlueprintResources/StandardMacros.IncrementInt` (`CapCharacter.vaccine` (stale `self.Box.OnComponentBeginOverlap` _ascap_character))
          (:`  `
            (`self.K2_DestroyActor`)))))))

(event `self.Box.OnComponentBeginOverlap`
  (params (OverlappedComponent :type "PrimitiveComponent Object Reference") (OtherActor :type "Actor Object Reference") (OtherComp :type "PrimitiveComponent Object Reference") (OtherBodyIndex :type Integer) (bFromSweep :type Boolean) (SweepResult :type "HitResult Structure (by ref)"))
  (bind _ascap_character (cast `CapCharacter` (`GameplayStatics.GetPlayerCharacter` 0)))
  (`self.EnableInput` (`GameplayStatics.GetPlayerController` 0))
  (bind _returnvalue (`|CreateWidget` "/Game/UI/HUD/PickupWidget2.PickupWidget2_C"))
  (bind _output_get (set `self.Widget Ref` _returnvalue))
  (`UserWidget.AddToViewport` _output_get 0)
  (goto _label :!via `Open`))

(event `self.Box.OnComponentEndOverlap`
  (params (OverlappedComponent :type "PrimitiveComponent Object Reference") (OtherActor :type "Actor Object Reference") (OtherComp :type "PrimitiveComponent Object Reference") (OtherBodyIndex :type Integer))
  (cast `CapCharacter` (`GameplayStatics.GetPlayerCharacter` 0))
  (`self.DisableInput` (`GameplayStatics.GetPlayerController` 0))
  (`Widget.RemoveFromParent` (stale `self.Box.OnComponentBeginOverlap` _returnvalue))
  (goto _label :!via `Close`))

(fn `UserConstructionScript`)